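; BP_SpawnableItem is an item actor that floats back and forth continuously around the game world.
; On BeginPlay it stores the root component's relative location, then a timeline drives that root by a scaled Offset vector added to the stored position.
; Forward and reverse playback restart each other on finish, forming an endless ping-pong motion.
; Overlap and Tick events are empty, so no pickup or spawning logic exists here.
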(event EventBeginPlay
  (bind _offset (Variables|Instance|Getoffset))
  (bind _defaultsceneroot (Variables|Default|GetDefaultSceneRoot))
  (Variables|Default|SetinitialPos (Variables|/Script/Engine.SceneComponent|GetRelativeLocation (Variables|Default|GetDefaultSceneRoot)))
  (bind _float (Timeline|FloatAnimation Play)
    (:Update
      (Transformation|SetRelativeLocation _defaultsceneroot (+ (* _float _offset) (Variables|Default|GetinitialPos)) false false))
    (:Finished
      (bind _float_2 (Timeline|Timeline ReverseFromEnd)
        (:Update
          (Transformation|SetRelativeLocation _defaultsceneroot (+ (* _float_2 _offset) (Variables|Default|GetinitialPos)) false false))
        (:Finished
          (Timeline|FloatAnimation PlayFromStart))))))

(event Collision|EventActorBeginOverlap
  (params (OtherActor :type Actor%20Object%20Reference)))

(event EventTick
  (params (DeltaSeconds :type Float%20%28single-precision%29)))

(fn ConstructionScript)