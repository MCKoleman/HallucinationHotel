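; Exit door actor for the Hallucination Hotel rooms that swings two hinges open when any actor overlaps it and closed when an overlap ends.
; Separate open and close timelines each stop the other and play from the start, driving hinge rotation, with Hinge1 negated to mirror Hinge2.
; BeginPlay also runs the close animation.
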(event Custom|OnDoorOpen
  (bind _hinge1 (Variables|Default|GetHinge1))
  ;[1 1 1] Animation
  (Utilities|FlowControl|Sequence
    (:then_0
      (bind _doorrotation (Timeline|Timeline_0 Stop)
        (:Update
          (Transformation|SetRelativeRotation _hinge1 (Class|KismetMathLibrary|QuatRotator (Class|KismetMathLibrary|QuatMakefromEuler _doorrotation)) false false)
          (Transformation|SetRelativeRotation _hinge1 (Class|KismetMathLibrary|NegateRotator (Class|KismetMathLibrary|QuatRotator (Class|KismetMathLibrary|QuatMakefromEuler _doorrotation))) false false))))
    (:then_1
      (bind _doorrotation_2 (Timeline|Timeline PlayFromStart)
        (:Update
          (Transformation|SetRelativeRotation _hinge1 (Class|KismetMathLibrary|QuatRotator (Class|KismetMathLibrary|QuatMakefromEuler _doorrotation_2)) false false)
          (Transformation|SetRelativeRotation _hinge1 (Class|KismetMathLibrary|NegateRotator (Class|KismetMathLibrary|QuatRotator (Class|KismetMathLibrary|QuatMakefromEuler _doorrotation_2))) false false))))))

(event Custom|OnDoorClose
  (bind _hinge1 (Variables|Default|GetHinge1))
  ;[1 1 1] Animation
  (Utilities|FlowControl|Sequence
    (:then_0
      (bind _doorrotation (Timeline|Timeline Stop)
        (:Update
          (Transformation|SetRelativeRotation _hinge1 (Class|KismetMathLibrary|QuatRotator (Class|KismetMathLibrary|QuatMakefromEuler _doorrotation)) false false)
          (Transformation|SetRelativeRotation _hinge1 (Class|KismetMathLibrary|NegateRotator (Class|KismetMathLibrary|QuatRotator (Class|KismetMathLibrary|QuatMakefromEuler _doorrotation))) false false))))
    (:then_1
      (bind _doorrotation_2 (Timeline|Timeline_0 PlayFromStart)
        (:Update
          (Transformation|SetRelativeRotation _hinge1 (Class|KismetMathLibrary|QuatRotator (Class|KismetMathLibrary|QuatMakefromEuler _doorrotation_2)) false false)
          (Transformation|SetRelativeRotation _hinge1 (Class|KismetMathLibrary|NegateRotator (Class|KismetMathLibrary|QuatRotator (Class|KismetMathLibrary|QuatMakefromEuler _doorrotation_2))) false false))))))

(event EventBeginPlay
  (CallFunction|OnDoorClose))

(event Collision|EventActorBeginOverlap
  (params (OtherActor :type Actor%20Object%20Reference))
  (CallFunction|OnDoorOpen))

(event Collision|EventActorEndOverlap
  (params (OtherActor :type Actor%20Object%20Reference))
  (CallFunction|OnDoorClose))

(fn ConstructionScript)