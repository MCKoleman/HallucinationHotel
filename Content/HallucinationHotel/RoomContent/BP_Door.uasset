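; BP_Door is a hinged door that opens when an actor overlaps it and closes when an overlap ends or play begins.
; Two timelines, DoorOpen and DoorClose, each stop the other and play from start, driving DoorHinge's relative rotation from vector tracks converted through quaternions.
; Overlaps are not filtered by actor type, and a Lerp01 rotation blend is left unconnected.
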(event Custom|OnDoorOpen
  ;[1 1 1] Animation
  (Utilities|FlowControl|Sequence
    (:then_0
      (bind _doorrotation (Timeline|DoorClose Stop)
        (:Update
          (Transformation|SetRelativeRotation (Variables|Default|GetDoorHinge) (Class|KismetMathLibrary|QuatRotator (Class|KismetMathLibrary|QuatMakefromEuler _doorrotation)) false false))))
    (:then_1
      (bind _doorrotation_2 (Timeline|DoorOpen PlayFromStart)
        (:Update
          (Transformation|SetRelativeRotation (Variables|Default|GetDoorHinge) (Class|KismetMathLibrary|QuatRotator (Class|KismetMathLibrary|QuatMakefromEuler _doorrotation_2)) false false))))))

(event Custom|OnDoorClose
  ;[1 1 1] Animation
  (Utilities|FlowControl|Sequence
    (:then_0
      (bind _doorrotation (Timeline|DoorOpen Stop)
        (:Update
          (Transformation|SetRelativeRotation (Variables|Default|GetDoorHinge) (Class|KismetMathLibrary|QuatRotator (Class|KismetMathLibrary|QuatMakefromEuler _doorrotation)) false false))))
    (:then_1
      (bind _doorrotation_2 (Timeline|DoorClose PlayFromStart)
        (:Update
          (Transformation|SetRelativeRotation (Variables|Default|GetDoorHinge) (Class|KismetMathLibrary|QuatRotator (Class|KismetMathLibrary|QuatMakefromEuler _doorrotation_2)) false false))))))

(event EventBeginPlay
  (CallFunction|OnDoorClose))

(event Collision|EventActorBeginOverlap
  (params (OtherActor :type Actor%20Object%20Reference))
  (CallFunction|OnDoorOpen))

(event Collision|EventActorEndOverlap
  (params (OtherActor :type Actor%20Object%20Reference))
  (CallFunction|OnDoorClose))

(fn ConstructionScript)