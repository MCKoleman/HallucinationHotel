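; BP_RoomLamp is a lamp actor for Hallucination Hotel rooms that switches a point light on and off.
; An IsLit flag holds the state, and the enable, disable and toggle events each update it before applying it to the PointLight's visibility.
; Any actor beginning an overlap with the lamp toggles the light, with no filter on the overlapping actor.
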(event Custom|onEnableLIght
  (Variables|Default|SetisLit true)
  (Rendering|SetVisibility (Variables|Default|GetPointLight) (Variables|Default|GetisLit) false))

(event Custom|onDisableLight
  (Variables|Default|SetisLit false)
  (Rendering|SetVisibility (Variables|Default|GetPointLight) (Variables|Default|GetisLit) false))

(event Custom|onToggleLight
  (Variables|Default|SetisLit (not (Variables|Default|GetisLit)))
  (Rendering|SetVisibility (Variables|Default|GetPointLight) (Variables|Default|GetisLit) false))

(event Collision|EventActorBeginOverlap
  (params (OtherActor :type Actor%20Object%20Reference))
  (CallFunction|OnToggleLight))

(fn ConstructionScript)